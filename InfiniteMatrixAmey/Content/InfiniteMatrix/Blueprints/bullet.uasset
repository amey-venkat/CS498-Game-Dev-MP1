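; Bullet projectile actor that flies along world X and destroys itself on any actor overlap or after a short lifetime.
; Each tick it moves with a swept world offset, adding a base speed to the player pawn's ForwardSpeed and a bonus scaled by PlayerScore.
; It reads both values live from BP_Player, so its speed tracks the player's speed and score.
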(event EventBeginPlay
  (Utilities|FlowControl|Delay 3.0)
  (Actor|DestroyActor))

(event Collision|EventActorBeginOverlap
  (params (OtherActor :type Actor%20Object%20Reference))
  (Actor|DestroyActor))

(event EventTick
  (params (DeltaSeconds :type Float%20%28single-precision%29))
  (bind _asbp_player (Utilities|Casting|CastToBP_Player (Game|Player|GetPlayerPawn 0)))
  (Transformation|AddActorWorldOffset (Math|Vector|MakeVector (* DeltaSeconds (+ 1e+03 (+ (Variables|/Game/InfiniteMatrix/Blueprints/BP_Player.BP_Player_C|GetForwardSpeed _asbp_player) (* 1e+01 (Math|Conversions|ToFloat(Integer) (Variables|/Game/InfiniteMatrix/Blueprints/BP_Player.BP_Player_C|GetPlayerScore _asbp_player)))))) 0.0 0.0) true))

(fn ConstructionScript)