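; Enemy actor that damages the player on contact and awards score when shot.
; Touching BP_Player calls its ProcessHit, refreshes the health bar and destroys the enemy.
; A bullet overlap destroys the enemy and raises player 0's score.
; Actor and Enemy component overlaps duplicate this logic, but the component's bullet branch writes score to the failed player cast instead of the fetched pawn.
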(event Custom|OnComponentBeginOverlap_Enemy
  (params (OverlappedComponent :type Primitive%20Component%20Object%20Reference) (OtherActor :type Actor%20Object%20Reference) (OtherComp :type Primitive%20Component%20Object%20Reference) (OtherBodyIndex :type Integer) (bFromSweep :type Boolean) (SweepResult :type Hit%20Result%20Structure%20%28by%20ref%29))
  (bind _asbp_player (Utilities|Casting|CastToBP_Player OtherActor)
    (:then
      (Default|ProcessHit _asbp_player)
      (Default|UpdateHealthbar (Variables|/Game/InfiniteMatrix/Blueprints/BP_Player.BP_Player_C|GetHealthHud _asbp_player) 0.0)
      (Actor|DestroyActor))
    (:CastFailed
      (Utilities|Casting|CastTobullet OtherActor)
      (bind _asbp_player_2 (Utilities|Casting|CastToBP_Player (Game|Player|GetPlayerPawn 0)))
      (Variables|/Game/InfiniteMatrix/Blueprints/BP_Player.BP_Player_C|SetPlayerScore _asbp_player (+ (Variables|/Game/InfiniteMatrix/Blueprints/BP_Player.BP_Player_C|GetPlayerScore _asbp_player_2) 25))
      (Actor|DestroyActor))))

(event EventBeginPlay)

(event Collision|EventActorBeginOverlap
  (params (OtherActor :type Actor%20Object%20Reference))
  (bind _asbp_player (Utilities|Casting|CastToBP_Player OtherActor)
    (:then
      (Default|ProcessHit _asbp_player)
      (Default|UpdateHealthbar (Variables|/Game/InfiniteMatrix/Blueprints/BP_Player.BP_Player_C|GetHealthHud _asbp_player) 0.0)
      (Actor|DestroyActor))
    (:CastFailed
      (Utilities|Casting|CastTobullet OtherActor)
      (bind _asbp_player_2 (Utilities|Casting|CastToBP_Player (Game|Player|GetPlayerPawn 0)))
      (Variables|/Game/InfiniteMatrix/Blueprints/BP_Player.BP_Player_C|SetPlayerScore _asbp_player_2 (+ (Variables|/Game/InfiniteMatrix/Blueprints/BP_Player.BP_Player_C|GetPlayerScore _asbp_player_2) 25))
      (Actor|DestroyActor))))

(event EventTick
  (params (DeltaSeconds :type Float%20%28single-precision%29)))

(fn ConstructionScript)